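; BP_level_floor is a floor segment actor that places one random obstacle on itself.
; The construction script gathers the left, center and right spawn component transforms and a list of three obstacle Blueprint classes.
; It then adds a child actor component at a randomly picked spawn point and sets its class to a random obstacle.
; The event graph contains only disabled placeholder events.
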(event EventBeginPlay)

(event Collision|EventActorBeginOverlap
  (params (OtherActor :type Actor%20Object%20Reference)))

(event EventTick
  (params (DeltaSeconds :type Float%20%28single-precision%29)))

(fn ConstructionScript
  (CallFunction|SetSpawnPoints)
  (CallFunction|SetObstacles)
  (CallFunction|SpawnObstacles))

(fn SetSpawnPoints
  (Variables|Default|SetSpawnPoints (Utilities|Array|MakeArray (Transformation|GetRelativeTransform (Variables|Default|GetSpawn%20L)) (Transformation|GetRelativeTransform (Variables|Default|GetSpawn%20Center)) (Transformation|GetRelativeTransform (Variables|Default|GetSpawn%20R)))))

(fn SetObstacles
  (Variables|Default|SetObstacles (Utilities|Array|MakeArray "/Game/Blueprints/BP_obstacle1.BP_obstacle1_C" "/Game/Blueprints/BP_obstacle2.BP_obstacle2_C" "/Game/Blueprints/BP_obstacle3.BP_obstacle3_C")))

(fn SpawnObstacles
  (bind _returnvalue (AddComponent|AddChildActorComponent false (.OutItem (Utilities|Array|Random (Variables|Default|GetSpawnPoints)))))
  (ChildActorComponent|SetChildActorClass _returnvalue (.OutItem (Utilities|Array|Random (Variables|Default|GetObstacles)))))