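; Spline mesh actor that grows a randomly winding path at runtime along its spline.
; The construction script lays a spline mesh component between each pair of existing points.
; From BeginPlay, a looping timer set by Frequency appends points with forward X and sideways Y random offsets scaled by NewSectionScale.
; Each step adds meshes for the last two segments so curves deform correctly, without removing the earlier mesh.
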(event Custom|Event%20NewSection
  (bind _lastpointindex (CallFunction|GetLastSplinePointIndex))
  ;[1 1 1] Creating a new point at set location
  (Spline|AddSplinePoint (Variables|Default|GetSpline) (+ (Spline|GetLocationatSplinePoint (Variables|Default|GetSpline) _lastpointindex "World") (Math|Vector|MakeVector (* (Math|Float|Clamp(Float) (Math|Random|RandomFloat) 0.5) (Variables|Default|GetNewSectionScale)) (* (- (* (Math|Random|RandomFloat) 2.0) 1.0) (Variables|Default|GetNewSectionScale)) 0.0)) "World" true)
  ;[1 1 1] Adding relevant meshes, we have to set the last to sections so they deform correctly
  (bind _lastpointindex_2 (CallFunction|GetLastSplinePointIndex))
  (CallFunction|AddMeshtoSplinePoint (- _lastpointindex_2 2) (- _lastpointindex_2 1))
  (bind _lastpointindex_3 (CallFunction|GetLastSplinePointIndex))
  (CallFunction|AddMeshtoSplinePoint (- _lastpointindex_3 1) _lastpointindex_3))

(event EventBeginPlay
  (Utilities|Time|SetTimerbyEvent (delegate Custom|Event%20NewSection) (/ 1.0 (Variables|Default|GetFrequency)) true))

(event Collision|EventActorBeginOverlap
  (params (OtherActor :type Actor%20Object%20Reference)))

(event EventTick
  (params (DeltaSeconds :type Float%20%28single-precision%29)))

(fn ConstructionScript
  (for _index (range 0 (- (Spline|GetNumberOfSplinePoints (Variables|Default|GetSpline)) 2))
    (CallFunction|AddMeshtoSplinePoint _index (+ _index 1))))

(fn AddMeshtoSplinePoint
  (params (Point%20index%20N :type Integer) (Point%20index%20N+1 :type Integer))
  (bind _spline (Variables|Default|GetSpline))
  (bind (_location _tangent) (Spline|GetLocationandTangentatSplinePoint _spline Point%20index%20N+1 "Local"))
  (bind (_location_2 _tangent_2) (Spline|GetLocationandTangentatSplinePoint _spline Point%20index%20N "Local"))
  (bind _returnvalue (AddComponent|AddSplineMeshComponent false))
  (SplineMesh|SetStartandEnd _returnvalue _location_2 _tangent_2 _location _tangent true :!class /Script/Engine.SplineMeshComponent)
  (Transformation|AttachComponentToComponent _returnvalue (Variables|Default|GetDefaultSceneRoot) "None" "KeepRelative" "KeepRelative" "KeepRelative" true)
  (Spline|UpdateSpline (Variables|Default|GetSpline)))

(fn GetLastSplinePointIndex
  (return (- (Spline|GetNumberOfSplinePoints (Variables|Default|GetSpline)) 1)))